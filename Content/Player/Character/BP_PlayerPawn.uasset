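; Player pawn that previews a single-bounce ricochet path from its facing direction, using debug-drawn sphere traces.
; Each Tick it sphere-traces forward on the Visibility channel, then traces again from the impact point along the direction reflected off the hit normal.
; The second trace runs without a hit check, and its result is unused.
; BeginPlay caches the forward vector, but Tick reads the live one instead.
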(event `self.ReceiveBeginPlay`
  (set `self.ForwVector` (`self.GetActorForwardVector`)))

(event `self.ReceiveTick`
  (params (DeltaSeconds :type "Float (single-precision)"))
  (bind _returnvalue (`self.GetActorForwardVector`))
  (bind _outhit (`KismetSystemLibrary.SphereTraceSingle` :`Start` (`self.K2_GetActorLocation`) :`End` (+ (`self.K2_GetActorLocation`) (* _returnvalue 2000.0)) :`Radius` 15.0 :`TraceChannel` "TraceTypeQuery1" :`DrawDebugType` "ForOneFrame"))
  (bind (_bblockinghit _binitialoverlap _time _distance _location _impactpoint _normal) (`GameplayStatics.BreakHitResult` _outhit))
  (`KismetSystemLibrary.SphereTraceSingle` :`Start` _impactpoint :`End` (+ _impactpoint (* (`KismetMathLibrary.GetReflectionVector` _returnvalue _normal) 1000.0)) :`Radius` 15.0 :`TraceChannel` "TraceTypeQuery1" :`DrawDebugType` "ForOneFrame"))

(fn `UserConstructionScript`)